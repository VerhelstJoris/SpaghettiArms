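; BP_Revolver is a gun Blueprint that spawns a BP_Projectile at its Arrow component's transform when the trigger is pulled.
; PullTrigger passes a DoOnce to call Fire, then sets a looping RoundsPerSecond-based timer back onto PullTrigger, whose repeat calls the DoOnce blocks.
; Releasetrigger resets the DoOnce and clears a timer named "Fire", which does not match the PullTrigger event timer.
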(event Custom|PullTrigger
  (Utilities|FlowControl|DoOnce false
    (:Completed
      (CallFunction|Fire)
      (Utilities|Time|SetTimerbyEvent (delegate Custom|PullTrigger) (/ 1.0 (Variables|Default|GetRoundsPerSecond)) true))))

(event Custom|Releasetrigger
  (Utilities|Time|ClearTimerbyFunctionName 0 "Fire")
  (Utilities|FlowControl|DoOnce false) ; enters at Reset
)

(event Custom|Fire
  (Game|SpawnActorfromClass "/Game/Blueprints/BP_Projectile.BP_Projectile_C" (Transformation|GetWorldTransform (Variables|Default|GetArrow)) "Undefined" 0 0))

(fn ConstructionScript)