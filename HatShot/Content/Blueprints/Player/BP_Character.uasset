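; BP_Character is a first-person player character with an attached gun and helper functions for movement, look and jumping.
; On BeginPlay it spawns a BP_BaseWeapon, stores it as CurrentWeapon and snaps it to the GripPoint socket on FPMesh.
; Movement follows the camera's forward and right vectors, look adds controller yaw and pitch, and jumping launches the character when CanJump passes.
; No input events in the file drive these functions.
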(event Custom|SpawnGun
  (bind _returnvalue (Components|GetOwner))
  ;[1 1 1] Spawn gun and attach it to the character
  (bind _returnvalue_2 (Game|SpawnActorfromClass "/Game/Blueprints/BP_BaseWeapon.BP_BaseWeapon_C" (Transformation|GetActorTransform _returnvalue) "AlwaysSpawn" _returnvalue 0))
  (bind _output_get (Variables|Default|SetCurrentWeapon _returnvalue_2))
  (Transformation|AttachComponentToComponent _output_get (Variables|Components|GetFP_Mesh) "GripPoint" "SnapToTarget" "SnapToTarget" "SnapToTarget" true))

(event EventBeginPlay
  (CallFunction|SpawnGun))

(fn ConstructionScript)

(fn ForwardMovement
  (params (force :type Float%20%28single-precision%29))
  (Pawn|Input|AddMovementInput (Math|Vector|GetForwardVector (Variables|Components|GetFirstperson_Camera)) force false))

(fn RightMovement
  (params (force :type Float%20%28single-precision%29))
  (Pawn|Input|AddMovementInput (Math|Vector|GetRightVector (Variables|Components|GetFirstperson_Camera)) force false))

(fn Turn
  (params (Yaw :type Float%20%28single-precision%29))
  (Pawn|Input|AddControllerYawInput Yaw))

(fn LookUp
  (params (Pitch :type Float%20%28single-precision%29))
  (Pawn|Input|AddControllerPitchInput Pitch))

(fn JumpMovement
  (params (JumpVelocity :type Vector))
  (if (Character|CanJump)
    (Character|LaunchCharacter JumpVelocity false false)))