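; Base first-person weapon Blueprint that handles firing, clip and reserve ammo, timed reloads, and creates its HUD widget on BeginPlay.
; Holding the trigger loops Fire and Recoil through a Delay, while a Tick-driven timer blocks re-pulls faster than the fire rate.
; Fire either spawns BP_Projectile at the muzzle or draws a beam tracer toward the camera trace, with no damage applied here.
; An empty clip triggers Reload when reserve ammo remains.
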(event Custom|PullTrigger
  (params (FP_camera :type Camera%20Component%20Object%20Reference) (FP_Character :type BP%20Character%20Object%20Reference))
  ;[1 1 1] Deciding when to fire
  (Variables|Private|Setfiring true)
  (if (not (Variables|Private|Getreloading))
    (if (== (Variables|Stats|GetDelayShotsTimer) 0.0)
      (if (> (Variables|Stats|GetCurrentAmmoInClip) 0) :!label _label
        (CallFunction|Fire FP_camera)
        (CallFunction|Recoil FP_Character)
        (Utilities|FlowControl|Delay (/ 1.0 (Variables|Stats|GetRoundsPerSecond)))
        (if (Variables|Private|Getfiring)
          (goto _label))
        (elif (> (Variables|Stats|GetCurrentTotalAmmo) 0)
          (CallFunction|Reload))))))

(event Custom|Recoil
  (params (FP_Character :type BP%20Character%20Object%20Reference))
  ;[1 1 1] Recoil
  (Pawn|Input|AddControllerPitchInput FP_Character (Variables|Stats|GetRecoilVertical)))

(event Custom|Releasetrigger
  ;[1 1 1] Deciding when to fire
  (Variables|Private|Setfiring false))

(event Custom|Reload
  ;[1 1 1] Reloading
  (if true
    (Variables|Private|Setreloading (!= (Variables|Stats|GetCurrentAmmoInClip) (Variables|Stats|GetAmmoPerClip)))
    (Utilities|FlowControl|Delay (Variables|Stats|GetReloadTime))
    (if (>= (Variables|Stats|GetCurrentTotalAmmo) (Variables|Stats|GetAmmoPerClip))
      (Variables|Stats|SetCurrentTotalAmmo (- (Variables|Stats|GetCurrentTotalAmmo) (- (Variables|Stats|GetAmmoPerClip) (Variables|Stats|GetCurrentAmmoInClip))))
      (Variables|Stats|SetCurrentAmmoInClip (Variables|Stats|GetAmmoPerClip))
      (Variables|Private|Setreloading false)
      (else
        (Variables|Stats|SetCurrentAmmoInClip (Variables|Stats|GetCurrentTotalAmmo))
        (Variables|Stats|SetCurrentTotalAmmo 0)))))

(event Custom|Fire
  (params (FP_Camera :type Camera%20Component%20Object%20Reference))
  (bind _returnvalue (Transformation|GetWorldLocation FP_Camera))
  (bind _returnvalue_2 (Math|Vector|GetForwardVector FP_Camera))
  (bind _muzzle (Variables|Default|GetMuzzle))
  (bind _returnvalue_3 (* _returnvalue_2 1.5e+04))
  (bind _returnvalue_4 (Transformation|GetWorldLocation _muzzle))
  (bind _returnvalue_5 (+ _returnvalue _returnvalue_3))
  ;[1 1 1] Fire
  (Variables|Stats|SetCurrentAmmoInClip (- (Variables|Stats|GetCurrentAmmoInClip) 1))
  (Variables|Stats|SetDelayShotsTimer (Utilities|Time|GetWorldDeltaSeconds))
  (bind _outhit (Collision|LineTraceByChannel _returnvalue _returnvalue_5 "TraceTypeQuery1" true 0 "None"))
  (if (Variables|Stats|GetShootsProjectiles)
    ;[1 1 1] Projectile
    (Game|SpawnActorfromClass "/Game/Blueprints/BP_Projectile.BP_Projectile_C" (Transformation|GetWorldTransform _muzzle) "Undefined" 0 0)
    (Audio|PlaySoundatLocation "/Game/FirstPerson_Template/FirstPerson/Audio/FirstPersonTemplateWeaponFire02.FirstPersonTemplateWeaponFire02" _returnvalue_4)
    (else
      ;[1 1 1] Raytrace Bullet
      (bind _returnvalue_6 (Effects|SpawnEmitteratLocation "/Game/Particles/P_BulletLine.P_BulletLine" "0, 0, 0"))
      (Class|ParticleSystemComponent|SetBeamSourcePoint _returnvalue_6 0 _returnvalue_4)
      (Audio|PlaySoundatLocation "/Game/FirstPerson_Template/FirstPerson/Audio/FirstPersonTemplateWeaponFire02.FirstPersonTemplateWeaponFire02" _returnvalue_4)
      (if (.bBlockingHit (Collision|BreakHitResult _outhit))
        (Class|ParticleSystemComponent|SetBeamTargetPoint _returnvalue_6 0 (.ImpactPoint (Collision|BreakHitResult _outhit)))
        (else
          (Class|ParticleSystemComponent|SetBeamTargetPoint _returnvalue_6 0 _returnvalue_5))))))

(event EventBeginPlay
  (Utilities|FlowControl|Sequence
    (:then_0
      (Variables|Stats|SetCurrentAmmoInClip (Variables|Stats|GetAmmoPerClip))
      (Variables|Stats|SetCurrentTotalAmmo (Variables|Stats|GetMaxAmmo)))
    (:then_1
      (bind _returnvalue (UserInterface|CreateWidget "/Game/HUD/Weapons/HUD_BaseWeapon.HUD_BaseWeapon_C"))
      (Variables|Components|SetHUD_Ref _returnvalue)
      (UserInterface|Viewport|AddtoViewport _returnvalue 0))))

(event EventTick
  (params (DeltaSeconds :type Float%20%28single-precision%29))
  ;[1 1 1] Deciding when to fire
  (if (!= (Variables|Stats|GetDelayShotsTimer) 0.0)
    (Variables|Stats|SetDelayShotsTimer (+ (Variables|Stats|GetDelayShotsTimer) (Utilities|Time|GetWorldDeltaSeconds)))
    (if (>= (Variables|Stats|GetDelayShotsTimer) (/ 1.0 (Variables|Stats|GetRoundsPerSecond)))
      (Variables|Stats|SetDelayShotsTimer 0.0))))

(fn ConstructionScript)