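; Weapon Blueprint for an automatic first-person gun with ammo, timed reloading, recoil and spread.
; PullTrigger loops shots at the fire rate until release, skipping sprinting and auto-reloading an empty clip.
; Each shot spawns Bullet_01 at the muzzle along camera rotation through RPCFire, with multicast sound, montage and randomized timeline-driven recoil.
; Spread grows per shot and decays on Tick within moving or standing limits, but is not applied to bullet rotation here.
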(event Custom|PullTrigger
  (params (FP_camera :type Camera%20Component%20Object%20Reference) (FP_Character :type First%20Person%20Character%20Object%20Reference))
  ;[1 1 1] Deciding when to fire
  (Variables|Private|Setfiring true)
  (if (not (Variables|Public|GetReloading))
    (if (== (Variables|Private|GetdelayShotsTimer) 0.0)
      (if (not (Variables|/Game/FirstPersonBP/Blueprints/FirstPersonCharacter.FirstPersonCharacter_C|GetisSprinting FP_Character)) :!label _label
        (if (> (Variables|Public|GetCurrentAmmoInClip) 0)
          (CallFunction|FIreWeapon FP_camera)
          (Animation|Montage|MontagePlay (Components|SkeletalMesh|GetAnimInstance (Variables|/Game/FirstPersonBP/Blueprints/FirstPersonCharacter.FirstPersonCharacter_C|GetMesh2P FP_Character)) "/Game/FirstPerson/Animations/FirstPersonFire_Montage.FirstPersonFire_Montage" 1.0 "MontageLength" 0.0)
          (CallFunction|IncreaseSpread (Variables|WeaponStats|GetSpreadIncreasePerShot))
          (CallFunction|Recoil FP_Character)
          (Utilities|FlowControl|Delay (/ 1.0 (Variables|WeaponStats|GetRoundsPerSecond)))
          (if (Variables|Private|Getfiring)
            (goto _label))
          (elif (> (Variables|Public|GetCurrentTotalAmmo) 0)
            (CallFunction|Reload)))))))

(event Custom|RPC%20Fire
  (bind _muzzle (Variables|Default|GetMuzzle))
  (bind _returnvalue (Transformation|GetWorldTransform _muzzle))
  (bind (_location _rotation _scale) (Math|Transform|BreakTransform _returnvalue))
  (CallFunction|MulticastFire)
  (Game|SpawnActorfromClass "/Game/FirstPersonBP/Blueprints/Bullet_01.Bullet_01_C" (Math|Transform|MakeTransform _location (Transformation|GetWorldRotation (stale Custom|FIreWeapon FP_Camera)) _scale) "Undefined" 0 0))

(event Custom|Recoil
  (params (Character :type First%20Person%20Character%20Object%20Reference))
  (bind _recoilhorizontalmax (Variables|WeaponStats|GetRecoilHorizontalMax))
  (bind _recoilhorizontalmax_2 (Variables|WeaponStats|GetRecoilHorizontalMax))
  (bind _recoilverticalmax (Variables|WeaponStats|GetRecoilVerticalMax))
  (bind _recoilverticalmax_2 (Variables|WeaponStats|GetRecoilVerticalMax))
  (bind _returnvalue (- 0.0 _recoilhorizontalmax))
  (bind _returnvalue_2 (* _recoilverticalmax 0.7))
  (bind _returnvalue_3 (Math|Random|RandomFloatinRange _returnvalue_2 _recoilverticalmax_2))
  (bind _returnvalue_4 (Math|Random|RandomFloatinRange _returnvalue _recoilhorizontalmax_2))
  ;[1 1 1] Recoil
  (Variables|Private|SetcurrentRecoilHorizontal _returnvalue_4)
  (Variables|Private|SettotalHorizontalRecoil (+ _returnvalue_4 (Variables|Private|GettotalHorizontalRecoil)))
  (Variables|Private|SetcurrentRecoilVertical _returnvalue_3)
  (Variables|Private|SettotalVerticalRecoil (+ _returnvalue_3 (Variables|Private|GettotalVerticalRecoil)))
  (bind _recoil (Timeline|RecoilTimeline PlayFromStart)
    (:Update
      (Pawn|Input|AddControllerPitchInput Character (* _recoil (Variables|Private|GetcurrentRecoilVertical)))
      (Pawn|Input|AddControllerYawInput Character (* _recoil (Variables|Private|GetcurrentRecoilHorizontal))))))

(event Custom|Multicast%20Fire
  (Audio|PlaySoundatLocation "/Game/FirstPerson/Audio/FirstPersonTemplateWeaponFire02.FirstPersonTemplateWeaponFire02" (Transformation|GetWorldLocation (Variables|Default|GetMuzzle))))

(event Custom|Releasetrigger
  ;[1 1 1] Deciding when to fire
  (Variables|Private|Setfiring false))

(event Custom|Reload
  ;[1 1 1] Reloading
  (if true
    (Variables|Public|SetReloading (!= (Variables|Public|GetCurrentAmmoInClip) (Variables|WeaponStats|GetAmmoPerClip)))
    (Utilities|FlowControl|Delay (Variables|WeaponStats|GetReloadTime))
    (if (>= (Variables|Public|GetCurrentTotalAmmo) (Variables|WeaponStats|GetAmmoPerClip))
      (Variables|Public|SetCurrentTotalAmmo (- (Variables|Public|GetCurrentTotalAmmo) (- (Variables|WeaponStats|GetAmmoPerClip) (Variables|Public|GetCurrentAmmoInClip))))
      (Variables|Public|SetCurrentAmmoInClip (Variables|WeaponStats|GetAmmoPerClip))
      (Variables|Public|SetReloading false)
      (else
        (Variables|Public|SetCurrentAmmoInClip (Variables|Public|GetCurrentTotalAmmo))
        (Variables|Public|SetCurrentTotalAmmo 0)))))

(event Custom|FIreWeapon
  (params (FP_Camera :type Camera%20Component%20Object%20Reference))
  ;[1 1 1] Fire
  (Variables|Public|SetCurrentAmmoInClip (- (Variables|Public|GetCurrentAmmoInClip) 1))
  (Variables|Private|SetdelayShotsTimer (Utilities|Time|GetWorldDeltaSeconds))
  (CallFunction|RPCFire))

(event EventBeginPlay
  (Utilities|FlowControl|Sequence
    (:then_0
      (Variables|Public|SetCurrentAmmoInClip (Variables|WeaponStats|GetAmmoPerClip))
      (Variables|Public|SetCurrentTotalAmmo (Variables|WeaponStats|GetMaxAmmo)))))

(event EventTick
  (params (DeltaSeconds :type Float%20%28single-precision%29))
  (Variables|Public|SetDeltaTime DeltaSeconds)
  (Utilities|FlowControl|Sequence
    (:then_0
      ;[1 1 1] delay between shots
      (if (!= (Variables|Private|GetdelayShotsTimer) 0.0)
        (Variables|Private|SetdelayShotsTimer (+ (Variables|Private|GetdelayShotsTimer) (Utilities|Time|GetWorldDeltaSeconds)))
        (if (>= (Variables|Private|GetdelayShotsTimer) (/ 1.0 (Variables|WeaponStats|GetRoundsPerSecond)))
          (Variables|Private|SetdelayShotsTimer 0.0))))
    (:then_1
      ;[1 1 1] Weapon Spread Decrease
      (CallFunction|DecreaseSpread (* (Variables|Public|GetDeltaTime) (Variables|WeaponStats|GetSpreadDecreaseSpeed))))))

(fn ConstructionScript)

(fn DecreaseSpread
  (params (DecreaseAmount :type Float%20%28single-precision%29))
  (if (Variables|Public|GetMoving)
    ;[1 1 1] while moving
    (if (<= (- (Variables|Public|GetCurrentSpread) DecreaseAmount) (Variables|WeaponStats|GetSpreadMinMovingHalfAngle))
      (Variables|Public|SetCurrentSpread (Variables|WeaponStats|GetSpreadMinMovingHalfAngle))
      (else
        (Variables|Public|SetCurrentSpread (- (Variables|Public|GetCurrentSpread) DecreaseAmount))))
    (else
      ;[1 1 1] while standing still
      (if (> (Variables|Public|GetCurrentSpread) (Variables|WeaponStats|GetSpreadMaxHalfAngle))
        (Variables|Public|SetCurrentSpread (Variables|WeaponStats|GetSpreadMaxHalfAngle))
        (elif (<= (- (Variables|Public|GetCurrentSpread) DecreaseAmount) (Variables|WeaponStats|GetSpreadMinHalfAngle))
          (Variables|Public|SetCurrentSpread (Variables|WeaponStats|GetSpreadMinHalfAngle))
          (else
            (Variables|Public|SetCurrentSpread (- (Variables|Public|GetCurrentSpread) DecreaseAmount))))))))

(fn IncreaseSpread
  (params (IncreaseAmount :type Float%20%28single-precision%29))
  (if (Variables|Public|GetMoving)
    ;[1 1 1] while moving
    (if (>= (+ IncreaseAmount (Variables|Public|GetCurrentSpread)) (Variables|WeaponStats|GetSpreadMaxMovingHalfAngle))
      (Variables|Public|SetCurrentSpread (Variables|WeaponStats|GetSpreadMaxMovingHalfAngle))
      (else
        (Variables|Public|SetCurrentSpread (+ IncreaseAmount (Variables|Public|GetCurrentSpread)))))
    (else
      ;[1 1 1] while standing still
      (if (>= (+ IncreaseAmount (Variables|Public|GetCurrentSpread)) (Variables|WeaponStats|GetSpreadMaxHalfAngle))
        (Variables|Public|SetCurrentSpread (Variables|WeaponStats|GetSpreadMaxHalfAngle))
        (else
          (Variables|Public|SetCurrentSpread (+ IncreaseAmount (Variables|Public|GetCurrentSpread))))))))

(fn SetMoving
  (params (moving :type Boolean))
  (Variables|Public|SetMoving moving))

(fn AddAmmo
  (params (Amount :type Integer))
  (Variables|Public|SetCurrentTotalAmmo (+ Amount (Variables|Public|GetCurrentTotalAmmo))))