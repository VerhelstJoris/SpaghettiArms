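; BP_Hurtzonre is a hazard zone that deals periodic damage to a FirstPersonCharacter inside its Zone component.
; Begin overlap stores the character and starts a looping CauseDamage timer at TickFrequency, which calls RPCTakeDamage with DamagePerTick and a zero hit location.
; End overlap by any FirstPersonCharacter clears the timer.
; Only one character reference is held, so the latest one to enter is the one damaged.
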(event OnComponentBeginOverlap(Zone)
  (params (OverlappedComponent :type Primitive%20Component%20Object%20Reference) (OtherActor :type Actor%20Object%20Reference) (OtherComp :type Primitive%20Component%20Object%20Reference) (OtherBodyIndex :type Integer) (bFromSweep :type Boolean) (SweepResult :type Hit%20Result%20Structure%20%28by%20ref%29))
  (bind _asfirst_person_character (Utilities|Casting|CastToFirstPersonCharacter OtherActor))
  (Variables|Default|SetFPCharReference _asfirst_person_character)
  (CallFunction|InZone))

(event OnComponentEndOverlap(Zone)
  (params (OverlappedComponent :type Primitive%20Component%20Object%20Reference) (OtherActor :type Actor%20Object%20Reference) (OtherComp :type Primitive%20Component%20Object%20Reference) (OtherBodyIndex :type Integer))
  (Utilities|Casting|CastToFirstPersonCharacter OtherActor)
  (CallFunction|OutOffZone))

(event Custom|InZone
  (bind _returnvalue (Utilities|Time|SetTimerbyFunctionName 0 "CauseDamage" (Variables|Variables|GetTickFrequency) true)))

(event Custom|OutOffZone
  (Utilities|Time|ClearandInvalidateTimerbyHandle (stale Custom|InZone _returnvalue)))

(fn ConstructionScript)

(fn CauseDamage
  (Default|RPCTakeDamage (Variables|Default|GetFPCharReference) (Variables|Variables|GetDamagePerTick) "0, 0, 0"))