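; BP_Obstacle1 is a shootable exploding hazard that loses HP on each Bullet_01 hit.
; At zero HP it runs an undelayed countdown loop with multicast sound and print, as both Delay nodes are disconnected.
; It then enables the DamageRadius collision, scaled at construction, to damage overlapping FirstPersonCharacters via RPCTakeDamage.
; A multicast explosion immediately follows, playing sound and particles and destroying the actor.
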(event OnComponentHit(Cylinder)
  (params (HitComponent :type Primitive%20Component%20Object%20Reference) (OtherActor :type Actor%20Object%20Reference) (OtherComp :type Primitive%20Component%20Object%20Reference) (NormalImpulse :type Vector :default "0, 0, 0") (Hit :type Hit%20Result%20Structure%20%28by%20ref%29))
  (Utilities|Casting|CastToBullet_01 OtherActor)
  (CallFunction|TakeDamage))

(event OnComponentHit(DamageRadius)
  (params (HitComponent :type Primitive%20Component%20Object%20Reference) (OtherActor :type Actor%20Object%20Reference) (OtherComp :type Primitive%20Component%20Object%20Reference) (NormalImpulse :type Vector :default "0, 0, 0") (Hit :type Hit%20Result%20Structure%20%28by%20ref%29))
  (Development|PrintString (Utilities|GetDisplayName OtherActor)))

(event OnComponentBeginOverlap(DamageRadius)
  (params (OverlappedComponent :type Primitive%20Component%20Object%20Reference) (OtherActor :type Actor%20Object%20Reference) (OtherComp :type Primitive%20Component%20Object%20Reference) (OtherBodyIndex :type Integer) (bFromSweep :type Boolean) (SweepResult :type Hit%20Result%20Structure%20%28by%20ref%29))
  (bind _asfirst_person_character (Utilities|Casting|CastToFirstPersonCharacter OtherActor))
  (Development|PrintText "Ouch")
  (Default|RPCTakeDamage _asfirst_person_character (Variables|Default|GetDamageCaused) "0, 0, 0"))

(event Custom|MulticastExplosion
  (params (SoundLocation :type Vector))
  (Audio|PlaySoundatLocation (Variables|Default|GetExplosionSound) SoundLocation "0, 0, 0" 1.5)
  (Effects|SpawnEmitteratLocation "/Game/Particle_effects/P_Shooting_Explosion_Barrel.P_Shooting_Explosion_Barrel" SoundLocation)
  (Actor|DestroyActor))

(event Custom|TakeDamage
  (bind _output_get (Variables|Default|SetHP (- (Variables|Default|GetHP) (Variables|Default|GetDamageTaken))))
  (if (< _output_get 0.1)
    (CallFunction|SelfDestruct)
    (else
      (Development|PrintString (Utilities|String|ToString(Float) _output_get)))))

(event Custom|SelfDestruct
  (bind _location (Variables|Default|GetLocation))
  (if (Variables|Default|GetKeepCountingDown) :!label _label
    (CallFunction|MulticastCountdown (Variables|Default|GetSelfDestructTimer) _location)
    (bind _result (Math|Float|DecrementFloat (Variables|Default|GetSelfDestructTimer))
      (:%20%20
        (bind _output_get (Variables|Default|SetSelfDestructTimer _result))
        (Variables|Default|SetKeepCountingDown (> _output_get 0.0))
        (goto _label)))
    (else
      (Collision|SetCollisionEnabled (Variables|Default|GetDamageRadius) "QueryOnly")
      (CallFunction|MulticastExplosion _location))))

(event Custom|MulticastCountdown
  (params (Count :type Float%20%28single-precision%29) (SoundLocation :type Vector))
  (Audio|PlaySoundatLocation (Variables|Default|GetCountdownSound) SoundLocation)
  (Development|PrintString (Utilities|String|ToString(Float) Count)))

(fn ConstructionScript
  (Collision|SetCollisionEnabled (Variables|Default|GetDamageRadius) "NoCollision")
  (Variables|Default|SetLocation (Transformation|GetActorLocation))
  (Transformation|SetWorldScale3D (Variables|Default|GetDamageRadius) (Variables|Default|GetAreaOfEffect)))