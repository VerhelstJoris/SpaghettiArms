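; BP_Saloon is a destructible saloon building that kills first-person characters touching its KillZone once it is destroyed.
; Hit passes damage to ServerTakeDamage, which reduces Health and calls a multicast destroy event when it runs out.
; That event disables actor collision, plays a sound, switches the KillZone from no collision to query-only, then removes the building after a short delay.
; Characters overlapping the active KillZone are destroyed outright.
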(event OnComponentBeginOverlap(KillZone)
  (params (OverlappedComponent :type Primitive%20Component%20Object%20Reference) (OtherActor :type Actor%20Object%20Reference) (OtherComp :type Primitive%20Component%20Object%20Reference) (OtherBodyIndex :type Integer) (bFromSweep :type Boolean) (SweepResult :type Hit%20Result%20Structure%20%28by%20ref%29))
  (bind _asfirst_person_character (Utilities|Casting|CastToFirstPersonCharacter OtherActor))
  (Actor|DestroyActor _asfirst_person_character))

(event Custom|Server%20Take%20Damage
  (params (DamageTaken :type Float%20%28single-precision%29))
  (bind _output_get (Variables|Default|SetHealth (- (Variables|Default|GetHealth) DamageTaken)))
  (if (not (> _output_get 0.0))
    (CallFunction|MulticastDestroy)))

(event Custom|Multicast%20destroy
  (Collision|SetActorEnableCollision false)
  (Audio|PlaySoundatLocation "/Game/Sounds/Smoke_Weed_Everyday_Sound_Effect.Smoke_Weed_Everyday_Sound_Effect" (Transformation|GetActorLocation))
  (Collision|SetCollisionEnabled (Variables|Default|GetKillZone) "QueryOnly")
  (Utilities|FlowControl|RetriggerableDelay 5.0)
  (Actor|DestroyActor))

(event EventBeginPlay)

(event Collision|EventActorBeginOverlap
  (params (OtherActor :type Actor%20Object%20Reference)))

(event EventTick
  (params (DeltaSeconds :type Float%20%28single-precision%29)))

(event Collision|EventHit
  (params (MyComp :type Primitive%20Component%20Object%20Reference) (Other :type Actor%20Object%20Reference) (OtherComp :type Primitive%20Component%20Object%20Reference) (bSelfMoved :type Boolean) (HitLocation :type Vector :default "0, 0, 0") (HitNormal :type Vector :default "0, 0, 0") (NormalImpulse :type Vector :default "0, 0, 0") (Hit :type Hit%20Result%20Structure%20%28by%20ref%29))
  (CallFunction|ServerTakeDamage (Variables|Default|GetDamageTaken)))

(fn ConstructionScript
  (Collision|SetCollisionEnabled (Variables|Default|GetKillZone) "NoCollision"))